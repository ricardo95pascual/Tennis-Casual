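; Game mode for a local two-player, ball-and-goal match that tracks score and declares the winner.
; BeginPlay creates a second local player, possesses and places both BP_Player pawns on opposite sides, creates the WBP_UI HUD and launches the first ball randomly.
; GoalEvent awards the point, destroys the ball and updates the HUD, then either respawns a ball after a delay, aimed toward the scorer's side, or shows victory at WinPoints.
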(event Custom|Spawn%20New%20Ball
  (params (isP1 :type Boolean))
  (Utilities|FlowControl|Delay 1.0)
  (CallFunction|SpawnBall isP1))

(event EventBeginPlay
  (Utilities|FlowControl|Sequence
    (:then_0
      (bind _returnvalue (Class|GameplayStatics|CreatePlayer 1))
      (bind _outactors (Actor|GetAllActorsOfClass "/Game/Blueprints/Player/CoreClass/BP_Player.BP_Player_C"))
      (Utilities|FlowControl|Sequence
        (:then_0
          ;[1 1 1] Poseer los jugadores
          (Pawn|Possess (Game|GetPlayerController 0) (Utilities|Array|Get(acopy) _outactors))
          (Default|SetIsPlayer2 (Utilities|Array|Get(acopy) _outactors) false)
          ;[1 1 1] Colocar en su sitio a los jugadores
          (Transformation|SetWorldTransform (Variables|/Script/Engine.Character|GetCapsuleComponent (Utilities|Array|Get(acopy) _outactors)) (Math|Transform|MakeTransform "-250.000000, 0,100.000000" "0, 0, 0" "1,1,1") false true)
          (Variables|Default|Set_P1 (Utilities|Array|Get(acopy) _outactors)))
        (:then_1
          (Pawn|Possess _returnvalue (Utilities|Array|Get(acopy) _outactors 1))
          (Default|SetIsPlayer2 (Utilities|Array|Get(acopy) _outactors 1) true)
          (Transformation|SetWorldTransform (Variables|/Script/Engine.Character|GetCapsuleComponent (Utilities|Array|Get(acopy) _outactors 1)) (Math|Transform|MakeTransform "1250.000000, 0,100.000000" "0, 0, 0" "1,1,1") false true)
          (bind _output_get (Variables|Default|Set_P2 (Utilities|Array|Get(acopy) _outactors 1))))))
    (:then_1
      (Variables|/Script/Engine.PlayerController|SetbShowMouseCursor (Game|GetPlayerController 0) false))
    (:then_2
      (bind _returnvalue_2 (UserInterface|CreateWidget "/Game/Blueprints/UI/WBP_UI.WBP_UI_C"))
      (bind _output_get_2 (Variables|Default|Set_HUD _returnvalue_2))
      (UserInterface|Viewport|AddtoViewport _output_get_2 0)
      (Variables|/Game/Blueprints/UI/WBP_UI.WBP_UI_C|SetPlayer1 (Variables|Default|Get_HUD) (Variables|Default|Get_P1))
      (Variables|/Game/Blueprints/UI/WBP_UI.WBP_UI_C|SetPlayer2 (Variables|Default|Get_HUD) (Variables|Default|Get_P2)))
    (:then_3
      (Default|SetGameMode (Variables|Default|Get_P1))
      (bind _outactors_2 (Actor|GetAllActorsOfClass "/Script/Engine.TriggerVolume")))
    (:then_4
      (Variables|Default|Set_PointsP1 0)
      (Variables|Default|Set_PointsP2 0)
      (CallFunction|SpawnNewBall (Math|Random|RandomBool)))))

(event EventTick
  (params (DeltaSeconds :type Float%20%28single-precision%29)))

(fn ConstructionScript)

(fn GoalEvent
  (params (IsP1 :type Boolean))
  (bind __winpoints (Variables|Default|Get_WinPoints))
  (if IsP1
    (Variables|Default|Set_PointsP1 (+ (Variables|Default|Get_PointsP1) 1))
    (else
      (Variables|Default|Set_PointsP2 (+ (Variables|Default|Get_PointsP2) 1))))
  (Actor|DestroyActor (Variables|Default|Get_GameBall))
  (CallFunction|UpdateHudScore)
  (if (and (< (Variables|Default|Get_PointsP1) __winpoints) (< (Variables|Default|Get_PointsP2) __winpoints))
    (CallFunction|SpawnNewBall IsP1)
    (else
      (CallFunction|Win))))

(fn SpawnBall
  (params (P1 :type Boolean))
  (bind _returnvalue (Math|Random|RandomFloatinRange -0.5 0.5))
  (Utilities|FlowControl|Sequence
    (:then_0
      (if P1
        (LocalVariables|SetSpawnDir (Math|Vector2D|MakeVector2D -1.0 _returnvalue))
        (else
          (LocalVariables|SetSpawnDir (Math|Vector2D|MakeVector2D 1.0 _returnvalue)))))
    (:then_1
      (bind _returnvalue_2 (Game|SpawnActorfromClass (Variables|Default|Get_GameBall_Spawn) (Math|Transform|MakeTransform "500.000000,0.000000,100.000000" "0, 0, 0" "1,1,1") "Undefined" 0 0))
      (Default|SetGameMode _returnvalue_2 self)
      (Variables|/Game/Blueprints/Ball/Core/BP_GameBall.BP_GameBall_C|Set_Direction _returnvalue_2 (LocalVariables|GetSpawnDir)))))

(fn UpdateHudScore
  (Default|UpdateScore (Variables|Default|Get_HUD) (Variables|Default|Get_PointsP1) (Variables|Default|Get_PointsP2)))

(fn Win
  (if (>= (Variables|Default|Get_PointsP1) (Variables|Default|Get_PointsP2))
    (LocalVariables|SetWinP1 true)
    (else
      (LocalVariables|SetWinP1 false)))
  (Default|Victory (Variables|Default|Get_HUD) (LocalVariables|GetWinP1))
  (Variables|/Script/Engine.PlayerController|SetbShowMouseCursor (Game|GetPlayerController 0) true))