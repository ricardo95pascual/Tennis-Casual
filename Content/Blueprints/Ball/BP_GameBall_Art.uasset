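; BP_GameBall_Art is the game ball's Blueprint layer for feedback such as hit audio, currently a scaffold with no effects implemented.
; SetNewDir, fired when the ball is struck, forwards direction, strength and element to the parent implementation, leaving room for additions afterward.
; GoalHit and WallHit are empty hooks, and unconnected switches on Strenght and Element are prepared for per-effectiveness and per-element sounds.
; Spanish comments mark these extension points.
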(event EventBeginPlay
  (|CallParentFunction) ; This node is disabled and will not be called.\nDrag off pins to build functionality.
)

(event Collision|EventActorBeginOverlap
  (params (OtherActor :type Actor%20Object%20Reference))
  (|CallParentFunction OtherActor) ; This node is disabled and will not be called.\nDrag off pins to build functionality.
)

(event EventTick
  (params (DeltaSeconds :type Float%20%28single-precision%29))
  (|CallParentFunction DeltaSeconds) ; This node is disabled and will not be called.\nDrag off pins to build functionality.
)

(event EventSetNewDir
  (params (Dir :type Vector%202D%20Structure) (Strenght :type EN_HitResult%20Enum :default "NewEnumerator0") (Element :type EN_Element%20Enum :default "NewEnumerator0"))
  (CallFunction|SetNewDir Dir Strenght Element) ; No borrar. Esto ejecuta mi código. Poned el vuestro despues
)

(event EventGoalHit
  ;[1 1 1] Aquí podeis poner el audio de golpe de bola con la pared
)

(event EventWallHit
  ;[1 1 1] Aquí podeis poner el audio de golpe de bola con la pared
)

(fn ConstructionScript
  (|CallParentFunction))