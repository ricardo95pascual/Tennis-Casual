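; BP_GameBall is a bouncing game ball that travels in 2D at a set speed and carries an elemental attribute shown by its color.
; Tick moves the Sphere with a swept offset; non-player hits flip one direction axis, chosen by comparing the hit location to the ball's center.
; SetNewDir sets direction, a strength-based speed and the element, then SetColor tints the dynamic material created in the Construction Script.
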(event EventBeginPlay
  (Variables|Default|Set_Direction (Math|Vector2D|Normalize2D (Math|Vector2D|MakeVector2D -1.0 0.5))))

(event Collision|EventActorBeginOverlap
  (params (OtherActor :type Actor%20Object%20Reference)))

(event EventTick
  (params (DeltaSeconds :type Float%20%28single-precision%29))
  (bind __speed (Variables|Default|Get_Speed))
  (bind __direction (Variables|Default|Get_Direction))
  (bind _returnvalue (Math|Vector2D|Normalize2D __direction))
  (bind _returnvalue_2 (* _returnvalue __speed))
  (bind _returnvalue_3 (* _returnvalue_2 DeltaSeconds))
  (Transformation|AddWorldOffset (Variables|Default|GetSphere) (Math|Vector|MakeVector (.x _returnvalue_3) (.y _returnvalue_3) 0.0) true false))

(event Collision|EventHit
  (params (MyComp :type Primitive%20Component%20Object%20Reference) (Other :type Actor%20Object%20Reference) (OtherComp :type Primitive%20Component%20Object%20Reference) (bSelfMoved :type Boolean) (HitLocation :type Vector :default "0, 0, 0") (HitNormal :type Vector :default "0, 0, 0") (NormalImpulse :type Vector :default "0, 0, 0") (Hit :type Hit%20Result%20Structure%20%28by%20ref%29))
  (Utilities|Casting|CastToBP_Player Other
    (:CastFailed
      (if (Math|Float|NearlyEqual(Float) (.x (Transformation|GetWorldLocation MyComp)) (.X (Math|Vector|BreakVector HitLocation)) 9.0)
        (Variables|Default|Set_Direction (Math|Vector2D|MakeVector2D (.x (Variables|Default|Get_Direction)) (* -1 (.y (Variables|Default|Get_Direction)))))
        (elif (Math|Float|NearlyEqual(Float) (.y (Transformation|GetWorldLocation MyComp)) (.Y (Math|Vector|BreakVector HitLocation)) 9.0)
          (Variables|Default|Set_Direction (Math|Vector2D|MakeVector2D (* -1 (.x (Variables|Default|Get_Direction))) (.y (Variables|Default|Get_Direction)))))))))

(fn ConstructionScript
  (bind __scale (Variables|Default|Get_Scale))
  (Transformation|SetWorldScale3D (Variables|Default|GetSphere) (Math|Vector|MakeVector __scale __scale __scale))
  (bind _returnvalue (Rendering|Material|CreateDynamicMaterialInstance (Variables|Default|GetSphere) 0 "/Game/Blueprints/Ball/MI_Ball.MI_Ball" :!class /Script/Engine.PrimitiveComponent))
  (Variables|Default|Set_Material _returnvalue)
  (CallFunction|SetColor))

(fn SetNewDir
  (params (Dir :type Vector%202D%20Structure) (Strenght :type EN_HitResult%20Enum :default "NewEnumerator0") (Element :type EN_Element%20Enum :default "NewEnumerator0"))
  (bind __speeds (Variables|Default|Get_Speeds))
  (Utilities|FlowControl|Sequence
    (:then_0
      (Variables|Default|Set_Direction (Math|Vector2D|Normalize2D Dir)))
    (:then_1
      (switch Utilities|FlowControl|Switch|SwitchonEN_HitResult Strenght
        (:NewEnumerator0
          (Variables|Default|Set_Speed (.x __speeds)))
        (:NewEnumerator1
          (Variables|Default|Set_Speed (.y __speeds)))
        (:NewEnumerator2
          (Variables|Default|Set_Speed (.z __speeds)))))
    (:then_2
      (Variables|Default|Set_Atribute Element)
      (CallFunction|SetColor))))

(fn SetColor
  (Utilities|FlowControl|Sequence
    (:then_0
      (switch Utilities|FlowControl|Switch|SwitchonEN_Element (Variables|Default|Get_Atribute)
        (:NewEnumerator0
          (LocalVariables|SetNewColor "(R=1.000000,G=0.000000,B=0.000000,A=1.000000)"))
        (:NewEnumerator1
          (LocalVariables|SetNewColor "(R=0.000000,G=0.000000,B=1.000000,A=1.000000)"))
        (:NewEnumerator2
          (LocalVariables|SetNewColor "(R=0.000000,G=1.000000,B=0.000000,A=1.000000)"))
        (:NewEnumerator3
          (LocalVariables|SetNewColor "(R=1.000000,G=1.000000,B=0.000000,A=1.000000)"))
        (:NewEnumerator5
          (LocalVariables|SetNewColor "(R=0.340000,G=0.000000,B=1.000000,A=1.000000)"))
        (:NewEnumerator6
          (LocalVariables|SetNewColor "(R=1.000000,G=1.000000,B=1.000000,A=1.000000)"))))
    (:then_1
      (Rendering|Material|SetVectorParameterValue (Variables|Default|Get_Material) "Color" (LocalVariables|GetNewColor) :!class /Script/Engine.MaterialInstanceDynamic))))