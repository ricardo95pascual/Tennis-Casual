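; Player character for a two-player ball game, moved every tick and able to hit the ball with three elemental attacks.
; Hit inputs lock steering, then after a delay sphere-trace for BP_GameBall, redirecting it along blended input and facing with strength and element from CompareElements.
; A successful hit swaps the used element with the pool's front and refreshes the GameMode's HUD.
; Random element setup is disconnected, and Player 2's numpad bindings are partial.
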(event Custom|HitStart
  (params (Element :type EN_Element%20Enum :default "NewEnumerator0") (Hit_Used :type EN_HitUsed%20Enum :default "NewEnumerator0"))
  ;[0 0 0] Golpeo de la bola
  ;;[1 1 1] Padre, lo del delay antes de golpear la bola
  (Utilities|FlowControl|Delay (Variables|BallHit|Get_TakeControlBeforeBallHit))
  (CallFunction|HitBall Element Hit_Used))

(event Custom|HitBall
  (params (Element :type EN_Element%20Enum :default "NewEnumerator0") (HitUsed :type EN_HitUsed%20Enum :default "NewEnumerator0"))
  (bind _returnvalue (Input|AxisValues|GetMove_X))
  (bind _returnvalue_2 (Input|AxisValues|GetMove_Y))
  (bind _capsulecomponent (Variables|Collision|GetCapsuleComponent))
  (bind __facingdirection (Variables|Default|Get_FacingDirection))
  (bind _returnvalue_3 (Transformation|GetWorldLocation _capsulecomponent))
  (bind _returnvalue_4 (Math|Vector2D|MakeVector2D _returnvalue _returnvalue_2))
  (bind _returnvalue_5 (Math|Vector2D|Normalize2D _returnvalue_4))
  (bind _returnvalue_6 (Math|Vector|Lerp(Vector) (Math|Vector|MakeVector (.x _returnvalue_5) (.y _returnvalue_5) 0.0) __facingdirection 0.5))
  ;[0 0 0] Golpeo de la bola
  (Utilities|FlowControl|Sequence
    (:then_0
      ;;[1 1 1] Lo de intentar golpear la bola
      (bind (_outhit _returnvalue_7) (Collision|SphereTraceForObjects _returnvalue_3 _returnvalue_3 (Variables|BallHit|Get_HitRange) (Utilities|Array|MakeArray "ObjectTypeQuery2") false 0 "ForDuration"))
      (if _returnvalue_7
        (bind _asbp_game_ball (Utilities|Casting|CastToBP_GameBall (.HitActor (Collision|BreakHitResult _outhit))))
        (CallFunction|UseElement HitUsed Element)
        (bind (_ballnewelement _hitresult) (CallFunction|CompareElements (Variables|/Game/Blueprints/Ball/BP_GameBall.BP_GameBall_C|Get_Atribute _asbp_game_ball) Element))
        ;;[1 1 1] Lo de cambiar la dirección a la bola
        (Default|SetNewDir _asbp_game_ball (Math|Vector2D|MakeVector2D (.x _returnvalue_6) (.y _returnvalue_6)) _hitresult _ballnewelement)))
    (:then_1
      ;;[1 1 1] Lo del delay despues de golpear la bola
      (Utilities|FlowControl|Delay (Variables|BallHit|Get_TakeControlAfterBallHit))
      (Variables|Movement|Set_isOnHit false))))

(event EventBeginPlay
  (Utilities|FlowControl|Sequence
    (:then_0
      (bind _asbpgm_my_game_mode (Utilities|Casting|CastToBPGM_MyGameMode (Game|GetGameMode)))
      (bind _output_get (Variables|GameLogic|Set_GameMode _asbpgm_my_game_mode))
      (bind _output_get_2 (Variables|GameLogic|Set_HUD (Variables|/Game/Blueprints/Game_Logic/BPGM_MyGameMode.BPGM_MyGameMode_C|Get_HUD _output_get)))
      (Default|UpdateHitButtonColors _output_get_2))))

(event Collision|EventActorBeginOverlap
  (params (OtherActor :type Actor%20Object%20Reference)))

(event EventTick
  (params (DeltaSeconds :type Float%20%28single-precision%29))
  (Movement|SetMovementInput))

(event Input|ActionEvents|InputActionHit_1
  (params (Key :type Key%20Structure))
  ;[0 0 0] Golpeo de la bola
  ;;[1 1 1] Padre, lo de los inputs
  (:Pressed
    (if (not (Variables|Movement|Get_isOnHit))
      (Variables|Movement|Set_isOnHit true)
      (CallFunction|HitStart (Variables|Default|Get_ElementA) "NewEnumerator0"))))

(event Input|ActionEvents|InputActionHit_2
  (params (Key :type Key%20Structure))
  ;[0 0 0] Golpeo de la bola
  ;;[1 1 1] Padre, lo de los inputs
  (:Pressed
    (if (not (Variables|Movement|Get_isOnHit))
      (Variables|Movement|Set_isOnHit true)
      (CallFunction|HitStart (Variables|Default|Get_ElementB) "NewEnumerator1"))))

(event Input|ActionEvents|InputActionHit_3
  (params (Key :type Key%20Structure))
  ;[0 0 0] Golpeo de la bola
  ;;[1 1 1] Padre, lo de los inputs
  (:Pressed
    (if (not (Variables|Movement|Get_isOnHit))
      (Variables|Movement|Set_isOnHit true)
      (CallFunction|HitStart (Variables|Default|Get_ElementC) "NewEnumerator2"))))

(event Input|KeyboardEvents|A
  (params (Key :type Key%20Structure)))

(event Input|KeyboardEvents|D
  (params (Key :type Key%20Structure)))

(event Input|KeyboardEvents|S
  (params (Key :type Key%20Structure)))

(event Input|KeyboardEvents|W
  (params (Key :type Key%20Structure)))

(event Input|KeyboardEvents|NumPadFour
  (params (Key :type Key%20Structure))
  ;[0 0 0] Golpeo de la bola
  ;;[1 1 1] Padre, lo de los inputs
  (:Pressed
    (if (Variables|Default|Get_IsPlayer2)
      (if (not (Variables|Movement|Get_isOnHit))
        (Variables|Movement|Set_isOnHit true)
        (CallFunction|HitStart (Variables|Default|Get_ElementB) "NewEnumerator1")))))

(event Input|KeyboardEvents|NumPadSix
  (params (Key :type Key%20Structure))
  ;[0 0 0] Golpeo de la bola
  ;;[1 1 1] Padre, lo de los inputs
  (:Pressed
    (if (Variables|Default|Get_IsPlayer2)
      _)))

(event Input|KeyboardEvents|NumPadTwo
  (params (Key :type Key%20Structure))
  ;[0 0 0] Golpeo de la bola
  ;;[1 1 1] Padre, lo de los inputs
  (:Pressed
    (if (Variables|Default|Get_IsPlayer2)
      (if (not (Variables|Movement|Get_isOnHit))
        (Variables|Movement|Set_isOnHit true)
        (CallFunction|HitStart (Variables|Default|Get_ElementA) "NewEnumerator0")))))

(fn ConstructionScript)

(fn SetElements
  (Utilities|FlowControl|Sequence))

(fn SetMovementInput
  (Utilities|FlowControl|Sequence
    (:then_0
      (if true
        ;[1 1 1] Ver si el input afecta a la dirección
        (if (not (Variables|Movement|Get_isOnHit))
          (Variables|Movement|Set_movementInput (Math|Vector2D|MakeVector2D (Input|AxisValues|GetMove_X) (Input|AxisValues|GetMove_Y))))))
    (:then_1
      ;[1 1 1] Lo de moverse
      (Class|PawnMovementComponent|AddInputVector (Variables|Character|GetCharacterMovement) (Math|Vector|MakeVector (.x (Variables|Movement|Get_movementInput)) (.y (Variables|Movement|Get_movementInput)) 0.0) false))))

(fn UseElement
  (params (HitUsed :type EN_HitUsed%20Enum :default "NewEnumerator0") (ElementUsed :type EN_Element%20Enum :default "NewEnumerator0"))
  (bind __elementremainingpool (Variables|Default|Get_ElementRemainingPool))
  (bind _output (Utilities|Array|Get(acopy) __elementremainingpool))
  (LocalVariables|SetUsedElement ElementUsed)
  (switch Utilities|FlowControl|Switch|SwitchonEN_HitUsed HitUsed
    (:NewEnumerator0
      (Variables|Default|Set_ElementA _output)
      (Utilities|Array|Add __elementremainingpool (LocalVariables|GetUsedElement)))
    (:NewEnumerator1
      (Variables|Default|Set_ElementB _output)
      (Utilities|Array|Add __elementremainingpool (LocalVariables|GetUsedElement)))
    (:NewEnumerator2
      (Variables|Default|Set_ElementC _output)
      (Utilities|Array|Add __elementremainingpool (LocalVariables|GetUsedElement))))
  (Utilities|Array|RemoveIndex __elementremainingpool)
  (Default|UpdateHitButtonColors (Variables|GameLogic|Get_HUD)))

(fn ShowInterfazChustera
  (bind _returnvalue (Utilities|Time|GetWorldDeltaSeconds))
  (Development|PrintString "----" true false "(R=0.000000,G=0.660000,B=1.000000,A=1.000000)" _returnvalue)
  (Development|PrintString (Utilities|String|Append "Right: " (Utilities|String|EnumtoString (Variables|Default|Get_ElementB))) true false "(R=0.000000,G=0.660000,B=1.000000,A=1.000000)" _returnvalue)
  (Development|PrintString (Utilities|String|Append "Down: " (Utilities|String|EnumtoString (Variables|Default|Get_ElementA))) true false "(R=0.000000,G=0.660000,B=1.000000,A=1.000000)" _returnvalue)
  (Development|PrintString (Utilities|String|Append "Left: " (Utilities|String|EnumtoString (Variables|Default|Get_ElementC))) true false "(R=0.000000,G=0.660000,B=1.000000,A=1.000000)" _returnvalue)
  (Development|PrintString "----" true false "(R=0.000000,G=0.660000,B=1.000000,A=1.000000)" _returnvalue))

(fn GetElements
  (return (Variables|Default|Get_ElementA) (Variables|Default|Get_ElementC) (Variables|Default|Get_ElementB)))

(fn SetIsPlayer2
  (params (isPlayer2? :type Boolean))
  (Variables|Default|Set_IsPlayer2 isPlayer2?)
  (if (not (Variables|Default|Get_IsPlayer2))
    (Variables|Default|Set_FacingDirection "1.000000, 0, 0")
    (else
      (Variables|Default|Set_FacingDirection "-1.000000, 0, 0"))))

(fn SetGameMode
  (bind _asbpgm_my_game_mode (Utilities|Casting|CastToBPGM_MyGameMode (Game|GetGameMode)))
  (bind _output_get (Variables|GameLogic|Set_GameMode _asbpgm_my_game_mode))
  (bind _output_get_2 (Variables|GameLogic|Set_HUD (Variables|/Game/Blueprints/Game_Logic/BPGM_MyGameMode.BPGM_MyGameMode_C|Get_HUD _output_get)))
  (Default|UpdateHitButtonColors _output_get_2))