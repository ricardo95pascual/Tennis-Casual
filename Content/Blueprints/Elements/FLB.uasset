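; Blueprint function library for the game's elements, resolving a hit between a ball and a player and mapping elements to indices.
; CompareElements uses nested switches to pick one of three hit results: Fire, Water and Leaf form a cycle, while Light and Dark counter each other.
; It returns that result with the player's element as the ball's new element; Neutral has no comparison branch.
; GetElementIndex converts each element, including Neutral, to an integer.
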(fn CompareElements
  (params (Ball_Element :type EN_Element%20Enum :default "NewEnumerator0") (Player_Element :type EN_Element%20Enum :default "NewEnumerator0"))
  (Utilities|FlowControl|Sequence
    (:then_0
      (LocalVariables|SetPlayer Player_Element)
      (switch Utilities|FlowControl|Switch|SwitchonEN_Element Ball_Element
        (:NewEnumerator0
          (switch Utilities|FlowControl|Switch|SwitchonEN_Element (LocalVariables|GetPlayer)
            (:NewEnumerator0
              (LocalVariables|SetOut_Hit "NewEnumerator1" :!label _label))
            (:NewEnumerator1
              (LocalVariables|SetOut_Hit "NewEnumerator0"))
            (:NewEnumerator2
              (LocalVariables|SetOut_Hit "NewEnumerator2"))
            (:NewEnumerator3
              (goto _label))
            (:NewEnumerator5
              (goto _label))))
        (:NewEnumerator1
          (switch Utilities|FlowControl|Switch|SwitchonEN_Element (LocalVariables|GetPlayer)
            (:NewEnumerator0
              (LocalVariables|SetOut_Hit "NewEnumerator2"))
            (:NewEnumerator1
              (LocalVariables|SetOut_Hit "NewEnumerator1" :!label _label_2))
            (:NewEnumerator2
              (LocalVariables|SetOut_Hit "NewEnumerator0"))
            (:NewEnumerator3
              (goto _label_2))
            (:NewEnumerator5
              (goto _label_2))))
        (:NewEnumerator2
          (switch Utilities|FlowControl|Switch|SwitchonEN_Element (LocalVariables|GetPlayer)
            (:NewEnumerator0
              (LocalVariables|SetOut_Hit "NewEnumerator0"))
            (:NewEnumerator1
              (LocalVariables|SetOut_Hit "NewEnumerator2"))
            (:NewEnumerator2
              (LocalVariables|SetOut_Hit "NewEnumerator1" :!label _label_3))
            (:NewEnumerator3
              (goto _label_3))
            (:NewEnumerator5
              (goto _label_3))))
        (:NewEnumerator3
          (switch Utilities|FlowControl|Switch|SwitchonEN_Element (LocalVariables|GetPlayer)
            (:NewEnumerator0
              (LocalVariables|SetOut_Hit "NewEnumerator1" :!label _label_4))
            (:NewEnumerator1
              (goto _label_4))
            (:NewEnumerator2
              (goto _label_4))
            (:NewEnumerator3
              (goto _label_4))
            (:NewEnumerator5
              (LocalVariables|SetOut_Hit "NewEnumerator0"))))
        (:NewEnumerator5
          (switch Utilities|FlowControl|Switch|SwitchonEN_Element (LocalVariables|GetPlayer)
            (:NewEnumerator0
              (LocalVariables|SetOut_Hit "NewEnumerator1" :!label _label_5))
            (:NewEnumerator1
              (goto _label_5))
            (:NewEnumerator2
              (goto _label_5))
            (:NewEnumerator3
              (LocalVariables|SetOut_Hit "NewEnumerator0"))
            (:NewEnumerator5
              (goto _label_5))))))
    (:then_1
      (return Player_Element (LocalVariables|GetOut_Hit)))))

(fn GetElementIndex
  (params (Element :type EN_Element%20Enum :default "NewEnumerator0"))
  (Utilities|FlowControl|Sequence
    (:then_0
      (switch Utilities|FlowControl|Switch|SwitchonEN_Element Element
        (:NewEnumerator0
          (LocalVariables|Setn 0))
        (:NewEnumerator1
          (LocalVariables|Setn 1))
        (:NewEnumerator2
          (LocalVariables|Setn 2))
        (:NewEnumerator3
          (LocalVariables|Setn 3))
        (:NewEnumerator5
          (LocalVariables|Setn 4))
        (:NewEnumerator6
          (LocalVariables|Setn 5))))
    (:then_1
      (return (LocalVariables|Getn)))))